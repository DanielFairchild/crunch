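; AI character Blueprint that feeds its behaviour tree blackboard and plays voice lines.
; Shortly after BeginPlay it writes its spawn, door and PC actors to the blackboard and plays a random opening line.
; Tick copies Health to the blackboard and, once it reaches zero, plays a random line from a second set a single time.
; While moving fast, a Delay and FlipFlop on Tick alternately add two audio components at a steady interval.
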(event EventBeginPlay
  (bind _audio (Variables|Default|GetAudio))
  (Utilities|FlowControl|Delay 0.2)
  (AI|Components|Blackboard|SetValueasObject (AI|GetBlackboard self) (Utilities|Name|MakeLiteralName "Spawn") (Variables|Default|GetSpawnActor))
  (AI|Components|Blackboard|SetValueasObject (AI|GetBlackboard self) (Utilities|Name|MakeLiteralName "Door") (Variables|Default|GetDoorActor))
  (AI|Components|Blackboard|SetValueasObject (AI|GetBlackboard self) (Utilities|Name|MakeLiteralName "PC") (Variables|Default|GetPCActor))
  (Variables|Default|SetPlayIndex (Math|Random|RandomIntegerinRange 0 8))
  (Audio|Components|Audio|SetSound _audio (Utilities|Select :Index (Variables|Default|GetPlayIndex) :Option%200 "/Game/Assets/Sounds/VoiceLines/All_of_this_just_works.All_of_this_just_works" :Option%201 "/Game/Assets/Sounds/VoiceLines/all_out_of_patience.all_out_of_patience" :Option%202 "/Game/Assets/Sounds/VoiceLines/demoing_the_game_at_e3.demoing_the_game_at_e3" :Option%203 "/Game/Assets/Sounds/VoiceLines/four_times_the_scale.four_times_the_scale" :Option%204 "/Game/Assets/Sounds/VoiceLines/four_times_the_scale_2.four_times_the_scale_2" :Option%205 "/Game/Assets/Sounds/VoiceLines/It_just_works.It_just_works" :Option%206 "/Game/Assets/Sounds/VoiceLines/It_just_works_2.It_just_works_2" :Option%207 "/Game/Assets/Sounds/VoiceLines/it_s_crunch_time.it_s_crunch_time" :Option%208 "/Game/Assets/Sounds/VoiceLines/it_s_release_time.it_s_release_time"))
  (Audio|Components|Audio|Play _audio 0.0))

(event EventTick
  (params (DeltaSeconds :type Float%20%28single-precision%29))
  (bind _audio (Variables|Default|GetAudio))
  (Utilities|FlowControl|Sequence
    (:then_0
      (AI|Components|Blackboard|SetValueasFloat (AI|GetBlackboard self) (Utilities|Name|MakeLiteralName "Health") (Variables|Default|GetHealth))
      (if (<= (Variables|Default|GetHealth) 0.0)
        (Utilities|FlowControl|DoOnce false
          (:Completed
            (Variables|Default|SetPlayIndex (Math|Random|RandomIntegerinRange 0 4))
            (Audio|Components|Audio|SetSound _audio (Utilities|Select :Index (Variables|Default|GetPlayIndex) :Option%200 "/Game/Assets/Sounds/VoiceLines/fine__you_have_24_hours.fine__you_have_24_hours" :Option%201 "/Game/Assets/Sounds/VoiceLines/Monika.Monika" :Option%202 "/Game/Assets/Sounds/VoiceLines/theres_no_bonuses.theres_no_bonuses" :Option%203 "/Game/Assets/Sounds/VoiceLines/The_fans_wont_be_happy_about_this.The_fans_wont_be_happy_about_this" :Option%204 "/Game/Assets/Sounds/VoiceLines/you_have_24_hours_2.you_have_24_hours_2"))
            (Audio|Components|Audio|Play _audio 0.0)))))
    (:then_1
      (if (> (Math|Vector|VectorLength (Transformation|GetVelocity)) 2e+02)
        (Utilities|FlowControl|Delay 0.6)
        (Utilities|FlowControl|FlipFlop
          (:A
            (AddComponent|AddAudioComponent false))
          (:B
            (AddComponent|AddAudioComponent false)))))))

(fn ConstructionScript)